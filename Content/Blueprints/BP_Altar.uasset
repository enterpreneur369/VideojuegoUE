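; BP_Altar is a puzzle altar that checks crates (BP_Caja) entering its Box trigger.
; A correct crate plays a button sound and runs a timeline that slides the BP_Puerta door found in the level along Z, with X and Y hard-coded.
; An incorrect crate deducts a life (Vidas) in BP_GameInstance and reloads Level_1.
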(event `self.Box.OnComponentBeginOverlap`
  (params (OverlappedComponent :type "PrimitiveComponent Object Reference") (OtherActor :type "Actor Object Reference") (OtherComp :type "PrimitiveComponent Object Reference") (OtherBodyIndex :type Integer) (bFromSweep :type Boolean) (SweepResult :type "HitResult Structure (by ref)"))
  (bind _asbp_caja (cast `/Game/Blueprints/BP_Caja` OtherActor))
  (if (`/Game/Blueprints/BP_Caja.correct` _asbp_caja)
    (bind _returnvalue (`GameplayStatics.GetActorOfClass` "/Game/Blueprints/BP_Puerta.BP_Puerta_C"))
    (`GameplayStatics.PlaySound2D` "/Game/Audio/Sfxs/Button.Button" 1.0 1.0 0.0 null null)
    (bind (_direction _traslacionpuerta) (`Timeline|TL_AbrirPuerta`)
      (:`Update`
        (`SceneComponent.K2_SetRelativeLocation` (`Actor.RootComponent` _returnvalue) (`KismetMathLibrary.MakeVector` 1188.0 3300.0 (+ (`self.InicialDoorPos`) (* _traslacionpuerta (`self.OffsetDoor`)))) false false)))
    (else
      (bind _asbp_game_instance (cast `/Game/BP_GameInstance` (`GameplayStatics.GetGameInstance`)))
      (set `/Game/BP_GameInstance.vidas` (- (`/Game/BP_GameInstance.vidas` _asbp_game_instance) 1) _asbp_game_instance)
      (`GameplayStatics.OpenLevel` "Level_1"))))

(fn `UserConstructionScript`)